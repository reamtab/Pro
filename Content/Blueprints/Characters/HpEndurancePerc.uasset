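; Character Blueprint logic that computes health and endurance fill ratios, likely for status display.
; CalcHpPerc divides current Hp by MaxHp, and CalcEndurPerc divides current Endur by MaxEndur.
; Both convert their values to float before dividing and return a fraction, with no clamping or zero-maximum guard.
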(fn CalcHpPerc
  ;[1 1 1] HP
  (bind _output_get (Variables|Default|SetHpPerc (/ (Math|Conversions|ToFloat(Integer) (Variables|Default|Gethp)) (Math|Conversions|ToFloat(Integer) (Variables|Default|GetMaxHp)))))
  (return _output_get))

(fn CalcEndurPerc
  ;[1 1 1] Endurance
  (bind _output_get (Variables|Default|SetEndurPerc (/ (Math|Conversions|ToFloat(Integer) (Variables|Default|GetEndur)) (Math|Conversions|ToFloat(Integer) (Variables|Default|GetMaxEndur)))))
  (return _output_get))